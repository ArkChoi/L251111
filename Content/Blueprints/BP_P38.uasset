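; BP_P38 is a player-controlled P-38 aircraft that steers by rotation and fires rockets through Enhanced Input.
; IA_Move applies local roll from its X axis and pitch from its Y axis, scaled by frame delta time.
; IA_Fire spawns a BP_Rocket at the Arrow component's world transform, with the plane as owner and instigator.
; The graph contains no forward movement or fire-rate limiting.
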(event Input|EnhancedActionEvents|EnhancedInputActionIA_Fire
  (params (ActionValue :type Boolean) (ElapsedSeconds :type Float%20%28double-precision%29) (TriggeredSeconds :type Float%20%28double-precision%29) (InputAction :type Input%20Action%20Object%20Reference :default "/Game/P_38Game/Input/IA_Fire.IA_Fire"))
  (bind _self self)
  (:Triggered
    (Game|SpawnActorfromClass "/Game/Blueprints/BP_Rocket.BP_Rocket_C" (Transformation|GetWorldTransform (Variables|Default|GetArrow)) "Undefined" "MultiplyWithRoot" _self _self)))

(event Input|EnhancedActionEvents|EnhancedInputActionIA_Move
  (params (ActionValue :type Vector%202D%20Structure) (ElapsedSeconds :type Float%20%28double-precision%29) (TriggeredSeconds :type Float%20%28double-precision%29) (InputAction :type Input%20Action%20Object%20Reference :default "/Game/P_38Game/Input/IA_Move.IA_Move"))
  (:Triggered
    (Transformation|AddActorLocalRotation (Math|Rotator|MakeRotator (* (.x ActionValue) (Utilities|Time|GetWorldDeltaSeconds) 6e+01) 0.0 0.0) false false)
    (Transformation|AddActorLocalRotation (Math|Rotator|MakeRotator 0.0 (* (.y ActionValue) (Utilities|Time|GetWorldDeltaSeconds) 6e+01) 0.0) false false)))

(fn ConstructionScript)