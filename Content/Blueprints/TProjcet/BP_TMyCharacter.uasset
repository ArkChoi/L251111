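; BP_TMyCharacter is a player character Blueprint that maps Enhanced Input actions to movement, running, camera look and jumping.
; Move input goes to either Run or Move depending on the IsRun flag, while the run action calls RunTrigger.
; Look input feeds pitch and yaw to Look, and jump input starts and stops jumping.
; The event graph only routes input, with Run, Move, Look and RunTrigger defined outside this file.
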(event Input|EnhancedActionEvents|EnhancedInputActionIA_Move
  (params (ActionValue :type Vector%202D%20Structure) (ElapsedSeconds :type Float%20%28double-precision%29) (TriggeredSeconds :type Float%20%28double-precision%29) (InputAction :type Input%20Action%20Object%20Reference :default "/Game/Input/Actions/IA_Move.IA_Move"))
  (:Triggered
    (if (Variables|Default|GetbIsRun)
      (Class|TMyCharacter|Run (.y ActionValue) (.x ActionValue))
      (else
        (Class|TMyCharacter|Move (.y ActionValue) (.x ActionValue))))))

(event Input|EnhancedActionEvents|EnhancedInputActionIA_Look
  (params (ActionValue :type Vector%202D%20Structure) (ElapsedSeconds :type Float%20%28double-precision%29) (TriggeredSeconds :type Float%20%28double-precision%29) (InputAction :type Input%20Action%20Object%20Reference :default "/Game/Input/Actions/IA_Look.IA_Look"))
  (Class|TMyCharacter|Look (.y ActionValue) (.x ActionValue)))

(event Input|EnhancedActionEvents|EnhancedInputActionIA_Jump
  (params (ActionValue :type Boolean) (ElapsedSeconds :type Float%20%28double-precision%29) (TriggeredSeconds :type Float%20%28double-precision%29) (InputAction :type Input%20Action%20Object%20Reference :default "/Game/Input/Actions/IA_Jump.IA_Jump"))
  (:Triggered
    (Character|Jump))
  (:Canceled
    (Character|StopJumping)))

(event Input|EnhancedActionEvents|EnhancedInputActionIA_Run
  (params (ActionValue :type Boolean) (ElapsedSeconds :type Float%20%28double-precision%29) (TriggeredSeconds :type Float%20%28double-precision%29) (InputAction :type Input%20Action%20Object%20Reference :default "/Game/Input/Actions/IA_Run.IA_Run"))
  (:Triggered
    (Class|TMyCharacter|RunTrigger)))

(fn ConstructionScript)